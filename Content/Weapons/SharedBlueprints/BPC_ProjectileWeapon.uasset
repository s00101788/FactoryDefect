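; Shared weapon Blueprint for projectile guns that extends the parent's OnFire by spawning an actor of class ProjectileType.
; FireProjectile places the projectile at the mesh's muzzle socket plus a fixed offset rotated by player 0's control rotation, which also sets its facing.
; The weapon is the spawned actor's owner and passes on its Instigator.
; The crosshair world position reaches FireProjectile but does not affect aim.
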(event EventBeginPlay)

(event Collision|EventActorBeginOverlap
  (params (OtherActor :type Actor%20Object%20Reference)))

(event EventOnFire
  (params (CrossHairWorldSpace :type Vector))
  (|CallParentFunction CrossHairWorldSpace)
  (CallFunction|FireProjectile CrossHairWorldSpace))

(event EventTick
  (params (DeltaSeconds :type Float%20%28single-precision%29)))

(fn ConstructionScript
  (|CallParentFunction))

(fn FireProjectile
  (params (CrosshairWorldSpace :type Vector))
  (bind _returnvalue (Game|Player|GetPlayerPawn 0))
  (bind _returnvalue_2 (Pawn|GetControlRotation _returnvalue :!class /Script/Engine.Pawn))
  (Game|SpawnActorfromClass (Variables|Default|GetProjectileType) (Math|Transform|MakeTransform (+ (Transformation|GetSocketLocation (Variables|Character|GetMesh) (Variables|Default|GetMuzzelSocket)) (Math|Vector|RotateVector "100.000000,-15.000000,30.000000" _returnvalue_2)) _returnvalue_2) "Undefined" self (Game|GetInstigator)))