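; Shared firing-weapon Blueprint that handles ammo, muzzle effects and hit feedback.
; OnFire checks ammo, then decrements it and plays the socket-attached muzzle flash and sound, or calls an empty no-ammo sound stub.
; Separate functions, not called here, loop over HitResult to apply point damage and spawn impact effects using BPAmmoBase data.
; OnFire does no tracing and leaves CrossHairWorldSpace unused; nothing here fills HitResult.
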(event Custom|OnFire
  (params (CrossHairWorldSpace :type Vector))
  ;[1 1 1] On Fire - Workflow when weapon is fired by a character
  (bind _canfire (CallFunction|CanWeaponFire))
  (if _canfire
    (CallFunction|DecrementAmmo)
    (CallFunction|PlayMuzzelFlash)
    (CallFunction|PlayFireSound)
    (else
      (CallFunction|PlayNoAmmoSound))))

(fn ConstructionScript
  (|CallParentFunction))

(fn CanWeaponFire
  (if (> (Variables|Attributes|GetAmmo) 0.0)
    (Variables|Default|SetCanFire? true)
    (else
      (Variables|Default|SetCanFire? false)))
  (return (Variables|Default|GetCanFire?)))

(fn DecrementAmmo
  (Variables|Attributes|SetAmmo (Math|Float|Clamp(Float) (- (Variables|Attributes|GetAmmo) 1.0) 0.0 (Variables|Attributes|GetMaxAmmo))))

(fn PlayNoAmmoSound)

(fn PlayMuzzelFlash
  (bind _muzzelsocket (Variables|Default|GetMuzzelSocket))
  (bind _scene (Variables|Default|GetScene))
  (Effects|SpawnEmitterAttached (Variables|Visuals|GetMuzzelFlash) _scene _muzzelsocket (Transformation|GetSocketLocation _scene _muzzelsocket) (Transformation|GetSocketRotation _scene _muzzelsocket) "KeepWorldPosition"))

(fn PlayFireSound
  (bind _mesh (Variables|Character|GetMesh))
  (bind _muzzelsocket (Variables|Default|GetMuzzelSocket))
  (Audio|SpawnSoundAttached (Variables|Default|GetFireSound) _mesh _muzzelsocket (Transformation|GetSocketLocation _mesh _muzzelsocket) (Transformation|GetSocketRotation _mesh _muzzelsocket) "KeepWorldPosition"))

(fn ApplyDamagetoHitActors
  (bind _returnvalue (Game|GetInstigatorController))
  (for _index (range 0 (- (Utilities|Array|Length (Variables|Default|GetHitResult)) 1))
    (Game|Damage|ApplyPointDamage (.HitActor (Collision|BreakHitResult (Utilities|Array|Get(acopy) (Variables|Default|GetHitResult) _index))) (Variables|/Game/Weapons/SharedBlueprints/BP_AmmoBase.BP_AmmoBase_C|GetBaseDamage (Variables|Default|GetBP_AmmoBase)) (Math|Rotator|GetRotationXVector (Math|Rotator|FindLookatRotation (.Location (Collision|BreakHitResult (Utilities|Array|Get(acopy) (Variables|Default|GetHitResult) _index))) (Transformation|GetActorLocation (Pawn|GetControlledPawn _returnvalue)))) (Utilities|Array|Get(acopy) (Variables|Default|GetHitResult) _index) _returnvalue self)))

(fn PlayImpactEffects
  (bind _bp_ammobase (Variables|Default|GetBP_AmmoBase))
  (for _index (range 0 (- (Utilities|Array|Length (Variables|Default|GetHitResult)) 1))
    (Effects|SpawnEmitteratLocation (Variables|/Game/Weapons/SharedBlueprints/BP_AmmoBase.BP_AmmoBase_C|GetImpactParticleSystem _bp_ammobase) (.Location (Collision|BreakHitResult (Utilities|Array|Get(acopy) (Variables|Default|GetHitResult) _index))))
    (Audio|SpawnSoundatLocation (Variables|/Game/Weapons/SharedBlueprints/BP_AmmoBase.BP_AmmoBase_C|GetImpactSound _bp_ammobase) (.Location (Collision|BreakHitResult (Utilities|Array|Get(acopy) (Variables|Default|GetHitResult) _index))) "0,0.000000, 0")))