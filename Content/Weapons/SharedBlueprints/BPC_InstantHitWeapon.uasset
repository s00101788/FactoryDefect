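; Instant-hit weapon Blueprint that extends a parent weapon's firing with hitscan traces and supports multiple traces per shot.
; When CanFire is true, DetermineHitObjects casts TracesUsed debug-drawn line traces from the player camera, randomised within a Spread cone out to Range.
; A hit triggers ApplyDamageToHitActors and PlayImpactEffects.
; HitResult only gains entries while the accumulated ObjectHit flag is false, and that flag is never reset here.
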(event EventBeginPlay)

(event Collision|EventActorBeginOverlap
  (params (OtherActor :type Actor%20Object%20Reference)))

(event EventOnFire
  (params (CrossHairWorldSpace :type Vector))
  (|CallParentFunction CrossHairWorldSpace)
  (if (Variables|Default|GetCanFire?)
    (bind _hitoccured_ (CallFunction|DetermineHitObjects (.WorldLocation (Game|Player|ConvertMouseLocationToWorldSpace (Game|GetPlayerController 0)))))
    (if _hitoccured_
      (CallFunction|ApplyDamagetoHitActors)
      (CallFunction|PlayImpactEffects))))

(event EventTick
  (params (DeltaSeconds :type Float%20%28single-precision%29)))

(fn ConstructionScript
  (|CallParentFunction))

(fn DetermineHitObjects
  (params (CrossHairWorldSpace :type Vector))
  (bind _returnvalue (Game|GetPlayerCameraManager 0))
  (bind _returnvalue_2 (Camera|GetCameraLocation _returnvalue))
  (Utilities|Array|Clear (Variables|Default|GetHitResult))
  (for _index (range 0 (- (Variables|Default|GetTracesUsed) 1))
    (bind (_outhit _returnvalue_3) (Collision|LineTraceByChannel _returnvalue_2 (+ _returnvalue_2 (* (Class|KismetMathLibrary|RandomUnitVectorinCone (Transformation|GetActorForwardVector _returnvalue) (Math|Trig|DegreesToRadians (Variables|Default|GetSpread))) (Variables|Default|GetRange))) "TraceTypeQuery1" false 0 "ForDuration"))
    (bind _output_get (Variables|Default|SetObjectHit? (or _returnvalue_3 (Variables|Default|GetObjectHit?))))
    (if (not _output_get)
      (Utilities|Array|AppendArray (Variables|Default|GetHitResult) (Utilities|Array|MakeArray _outhit))))
  (return (Variables|Default|GetObjectHit?)))