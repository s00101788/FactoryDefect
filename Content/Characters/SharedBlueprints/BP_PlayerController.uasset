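; Shared player controller that handles primary weapon firing for BPC_GunFighter pawns and calls PlaySound2D on BeginPlay.
; Fire input passes a crosshair location to the weapon's OnFire, but only when FirstPerson is false, despite the first-person comment.
; GetCrosshairLocation multiplies, rather than adds, FPCamera location by forward vector times weapon range, without tracing.
; An unfinished FlipFlop camera swap is left disconnected.
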(event EventTick
  (params (DeltaSeconds :type Float%20%28single-precision%29))
  ;[1 1 1] Attempt at Camera Swap
)

(event EventBeginPlay
  ;[1 1 1] Start Music when playing
  (Audio|PlaySound2D 0))

(event Input|ActionEvents|InputActionFirePrimaryWeapon
  (params (Key :type Key%20Structure :default "AnyKey"))
  (bind _returnvalue (Pawn|GetControlledPawn))
  (bind _asbpc_gun_fighter (Utilities|Casting|CastToBPC_GunFighter _returnvalue))
  ;[1 1 1] 1st Person Shooting - This means i can only shoot in first person it also give me the crosshair location
  (:Pressed
    (Utilities|IsValid _returnvalue
      (:Is%20Valid
        (if (not (Variables|/Game/Characters/SharedBlueprints/BPC_PlayerCharacter.BPC_PlayerCharacter_C|GetFirstPerson? _asbpc_gun_fighter))
          (bind _crosshairworldspace (CallFunction|GetCrosshairLocation))
          (Default|OnFire (Variables|/Game/Characters/SharedBlueprints/BPC_GunFighter.BPC_GunFighter_C|GetPrimaryWeapon _asbpc_gun_fighter) _crosshairworldspace))))))

(event Input|KeyboardEvents|C
  (params (Key :type Key%20Structure :default "AnyKey"))
  ;[1 1 1] Attempt at Camera Swap
)

(fn ConstructionScript)

(fn GetCrosshairLocation
  (bind _asbpc_gun_fighter (Utilities|Casting|CastToBPC_GunFighter (Game|GetPlayerCharacter 0)))
  (return (* (Transformation|GetWorldLocation (Variables|/Game/Characters/SharedBlueprints/BPC_PlayerCharacter.BPC_PlayerCharacter_C|GetFP_Camera _asbpc_gun_fighter)) (* (Math|Rotator|GetRotationXVector (Transformation|GetWorldRotation (Variables|/Game/Characters/SharedBlueprints/BPC_PlayerCharacter.BPC_PlayerCharacter_C|GetFP_Camera _asbpc_gun_fighter))) (Variables|/Game/Weapons/SharedBlueprints/BP_BaseWeapon.BP_BaseWeapon_C|GetRange (Variables|/Game/Characters/SharedBlueprints/BPC_GunFighter.BPC_GunFighter_C|GetPrimaryWeapon _asbpc_gun_fighter))))))