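; BPC_PlayerCharacter is a player character Blueprint that toggles between first-person and third-person views.
; A hardcoded C key press drives a FlipFlop that activates one of FollowCamera and FPCamera and deactivates the other.
; The FirstPerson flag reads inverted: it is true while FollowCamera is active and false while FPCamera is active.
; BeginPlay, overlap and Tick are unused, and the construction script only calls its parent.
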(event EventBeginPlay)

(event Collision|EventActorBeginOverlap
  (params (OtherActor :type Actor%20Object%20Reference)))

(event EventTick
  (params (DeltaSeconds :type Float%20%28single-precision%29)))

(event Input|KeyboardEvents|C
  (params (Key :type Key%20Structure :default "AnyKey"))
  (bind _self self)
  (bind _followcamera (Variables|Default|GetFollowCamera))
  (bind _fp_camera (Variables|Default|GetFP_Camera))
  ;[1 1 1] Perspective Swap - Via the C button implaments a swap between 1st and 3rd person views
  (:Pressed
    (Utilities|FlowControl|FlipFlop
      (:A
        (Components|Activation|SetActive _followcamera true false)
        (Components|Activation|SetActive _fp_camera false false)
        (Variables|BPC_PlayerCharacter_C|SetFirstPerson? _self true))
      (:B
        (Components|Activation|SetActive _fp_camera true false)
        (Components|Activation|SetActive _followcamera false false)
        (Variables|BPC_PlayerCharacter_C|SetFirstPerson? _self false)))))

(fn ConstructionScript
  (|CallParentFunction))