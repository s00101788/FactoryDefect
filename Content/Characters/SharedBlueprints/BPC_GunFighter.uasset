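; Shared gunfighter character Blueprint that spawns with a starting weapon and fires debug line traces on input.
; BeginPlay spawns the weapon at the mesh's Gun_Socket, attaches it, stores it as PrimaryWeapon and fills its ammo with one new clip.
; N press or left mouse release runs a visibility trace, scaling location plus forward vector together by MaxShootDistance for its end point.
; The hit result is unused, and firing consumes no ammo.
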(event EventBeginPlay
  (bind _self self)
  (bind _returnvalue (Game|SpawnActorfromClass (Variables|Default|GetStartingWeapon) (Transformation|GetSocketTransform (Variables|Character|GetMesh) "Gun_Socket" "RTS_World") "Undefined" _self _self))
  (Class|Actor|AttachRootComponenttoActor _returnvalue _self "Gun_Socket" "KeepWorldPosition" true)
  (Variables|Weapons|SetPrimaryWeapon _returnvalue)
  (Variables|/Game/Weapons/SharedBlueprints/BPC_FiringWeapon.BPC_FiringWeapon_C|SetAmmo (Variables|Weapons|GetPrimaryWeapon) (Variables|/Game/Weapons/SharedBlueprints/BP_AmmoBase.BP_AmmoBase_C|GetAmountInNewClip (Variables|/Game/Weapons/SharedBlueprints/BPC_FiringWeapon.BPC_FiringWeapon_C|GetBP_AmmoBase (Variables|Weapons|GetPrimaryWeapon)))))

(event Collision|EventActorBeginOverlap
  (params (OtherActor :type Actor%20Object%20Reference)))

(event EventTick
  (params (DeltaSeconds :type Float%20%28single-precision%29)))

(event Input|MouseEvents|LeftMouseButton
  (params (Key :type Key%20Structure :default "AnyKey"))
  (bind _returnvalue (Transformation|GetActorLocation))
  (:Released
    (bind _outhit (Collision|LineTraceByChannel _returnvalue (* (+ _returnvalue (Transformation|GetActorForwardVector)) (Variables|Default|GetMaxShootDistance)) "TraceTypeQuery1" false 0 "ForDuration"))))

(event Input|KeyboardEvents|N
  (params (Key :type Key%20Structure :default "AnyKey"))
  (bind _returnvalue (Transformation|GetActorLocation))
  (:Pressed
    (bind _outhit (Collision|LineTraceByChannel _returnvalue (* (+ _returnvalue (Transformation|GetActorForwardVector)) (Variables|Default|GetMaxShootDistance)) "TraceTypeQuery1" false 0 "ForDuration"))))

(fn ConstructionScript
  (|CallParentFunction))